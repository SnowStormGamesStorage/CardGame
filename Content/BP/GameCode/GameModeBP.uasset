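; Game mode for a two-player card game that sets up shuffled decks and handles turn counting and card draws.
; BeginPlay copies both decks from the game instance, shuffles them and clears the hands.
; DrawCards serves only Player 1, checking the hand limit, moving a card via AddCard and adding a HandCard widget to the HUD.
; The debug printouts and alternating two-player deal loop are disconnected.
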(event Custom|UpdateTurn
  ;[1 1 1] Update turns
  (Variables|Default|SetTurn (+ (Variables|Default|GetTurn) 1))
  (Development|PrintString (Utilities|String|ToString(Integer) 0)))

(event Custom|InitializeDecks
  (bind _mygameinstance (Variables|Default|GetMyGameInstance))
  ;[1 1 1] Set up Deck and Shuffle
  (Variables|Default|SetPlayer1ActiveDeck (Variables|/Game/BP/GameCode/Mygameinstance.Mygameinstance_C|GetPlayer1GameDeck _mygameinstance))
  (Variables|Default|SetPlayer2ActiveDeck (Variables|/Game/BP/GameCode/Mygameinstance.Mygameinstance_C|GetPlayer2GameDeck _mygameinstance))
  (Utilities|Array|Shuffle (Variables|Default|GetPlayer1ActiveDeck))
  (Utilities|Array|Shuffle (Variables|Default|GetPlayer2ActiveDeck))
  (Utilities|Array|Clear (Variables|Default|GetPlayer1Hand))
  (Utilities|Array|Clear (Variables|Default|GetPlayer2Hand))
  (Development|PrintString "DeckShuffled"))

(event Custom|InitializeAll
  ;[1 1 1] Set up first turn and initialize decks
  (Variables|Default|SetTurn 1)
  (CallFunction|InitializeDecks))

(event Custom|DrawCards
  ;[1 1 1] Draw one Card for a normal turn
  (CallFunction|DrawOneCard (Variables|Default|GetPlayer1ActiveDeck) (Variables|Default|GetPlayer1Hand)))

(event Custom|DrawOneCard
  (params (CurrentPlayerDeck :type Array%20of%20Hand%20Card%20Object%20References) (CurrentPlayerHand :type Array%20of%20Hand%20Card%20Object%20References))
  ;[1 1 1] Draw one Card for a normal turn
  (bind _isfull (CallFunction|Fullhand? CurrentPlayerHand (Variables|Default|GetNumberofCardsPerPlayer)))
  (if _isfull
    (CallFunction|FullHandWarning)
    (else
      (bind _cardtoload (CallFunction|AddCard CurrentPlayerHand CurrentPlayerDeck))
      (bind _returnvalue (UserInterface|CreateWidget "/Game/Widgets/HandCard.HandCard_C"))
      (Variables|/Game/Widgets/HandCard.HandCard_C|SetName _returnvalue (Utilities|String|StringToName (.Name (Utilities|Struct|BreakCardStructure (Variables|/Game/Widgets/HandCard.HandCard_C|GetCardData _cardtoload)))))
      (Variables|/Game/Widgets/HandCard.HandCard_C|SetCardData _returnvalue (Variables|/Game/Widgets/HandCard.HandCard_C|GetCardData _cardtoload))
      (Widget|Panel|AddChild (Variables|/Game/Widgets/MYHUD.MYHUD_C|GetPlayer1Hand (Variables|Default|GetMYHUD_REF)) _returnvalue))))

(event Custom|FullHandWarning
  ;[1 1 1] Draw one Card for a normal turn
  (Development|PrintString "HandIsFull"))

(event Custom|Break
  ;[1 1 1] Handling Cards from Live Deck
  (bind _index (Utilities|FlowControl|ForLoopwithBreak 0 (- (* (Variables|Default|GetNumberofCardsPerPlayer) 2) 1)) ; enters at Break
    (:LoopBody
      (Utilities|FlowControl|FlipFlop
        (:A
          (bind _isfull (CallFunction|Fullhand? (Variables|Default|GetPlayer1Hand) 3))
          (if _isfull
            (CallFunction|FullHandWarning :!label _label)
            (else
              (CallFunction|AddCard (Variables|Default|GetPlayer1ActiveDeck) 0 _index)
              (Variables|Default|SetPlayer1ActiveDeck 0)
              (Variables|Default|SetPlayer1Hand 0))))
        (:B
          (bind _isfull_2 (CallFunction|Fullhand? (Variables|Default|GetPlayer2Hand) 3))
          (if _isfull_2
            (goto _label)
            (else
              (CallFunction|AddCard (Variables|Default|GetPlayer2ActiveDeck) 0 _index)
              (Variables|Default|SetPlayer2ActiveDeck 0)
              (Variables|Default|SetPlayer2Hand 0))))))))

(event EventBeginPlay
  ;[1 1 1] Begin Play
  (bind _asmygameinstance (Utilities|Casting|CastToMygameinstance (Game|GetGameInstance))
    (:then
      (Variables|Default|SetMyGameInstance _asmygameinstance)
      (CallFunction|InitializeAll))
    (:CastFailed
      (Development|PrintString "CannotFindGameInstance" true true "(R=0.000000,G=0.660000,B=1.000000,A=1.000000)" 1e+01))))

(fn ConstructionScript)

(fn Fullhand?
  (params (Hand :type Array%20of%20Hand%20Card%20Object%20References) (NumberofCards :type Integer))
  (bind _returnvalue (Utilities|Array|Length Hand))
  (Development|PrintString (Utilities|String|ToString(Text) (Utilities|Text|FormatText "currenthandsize {A}" _returnvalue)) true true "(R=0.000000,G=0.660000,B=1.000000,A=1.000000)" 5.0)
  (if (>= _returnvalue NumberofCards)
    (return true)
    (else
      (return false))))

(fn AddCard
  (params (DeckHandIn :type Array%20of%20Hand%20Card%20Object%20References) (ActiveDeckIn :type Array%20of%20Hand%20Card%20Object%20References) (Index :type Integer))
  ;[1 1 1] Create local to save changes.
  (LocalVariables|SetDeckHandLocal DeckHandIn)
  (bind _output_get (LocalVariables|SetActiveDeckLocal ActiveDeckIn))
  (Utilities|Array|Add (LocalVariables|GetDeckHandLocal) (Utilities|Array|Get(acopy) _output_get Index))
  (Utilities|Array|RemoveItem (LocalVariables|GetActiveDeckLocal) (Utilities|Array|Get(acopy) _output_get Index))
  (return (LocalVariables|GetDeckHandLocal) (LocalVariables|GetActiveDeckLocal) (Utilities|Array|Get(acopy) _output_get Index)))